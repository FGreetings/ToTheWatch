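; BP_CannotMoveArea is a box trigger volume that slows human characters while they are inside it, rather than fully stopping them.
; Overlap events cast the other actor to BP_BaseHuman and lower its walk speed on entry, then set a hardcoded normal speed on exit instead of restoring the previous value.
; The construction script applies the BoxScale variable to the box's world scale to size the area.
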(event `self.Box.OnComponentBeginOverlap`
  (params (OverlappedComponent :type "PrimitiveComponent Object Reference") (OtherActor :type "Actor Object Reference") (OtherComp :type "PrimitiveComponent Object Reference") (OtherBodyIndex :type Integer) (bFromSweep :type Boolean) (SweepResult :type "HitResult Structure (by ref)"))
  (bind _asbp_base_human (cast `/Game/BluePrints/BP_BaseHuman` OtherActor))
  (set `CharacterMovementComponent.MaxWalkSpeed` 100.0 (`Character.CharacterMovement` _asbp_base_human)))

(event `self.Box.OnComponentEndOverlap`
  (params (OverlappedComponent :type "PrimitiveComponent Object Reference") (OtherActor :type "Actor Object Reference") (OtherComp :type "PrimitiveComponent Object Reference") (OtherBodyIndex :type Integer))
  (bind _asbp_base_human (cast `/Game/BluePrints/BP_BaseHuman` OtherActor))
  (set `CharacterMovementComponent.MaxWalkSpeed` 600.0 (`Character.CharacterMovement` _asbp_base_human)))

(fn `UserConstructionScript`
  (`SceneComponent.SetWorldScale3D` (`self.Box`) (`self.BoxScale`)))