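; Trigger volume that drops a short sequence of falling rocks when a BP_BaseHuman actor enters its Box.
; The overlap spawns three BP_RandomRocks at separate fall locations, staggered by short delays and scaled up.
; CanSpawn blocks re-entry during the delays and stays false after the last spawn, so a completed sequence does not repeat.
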(event `self.Box.OnComponentBeginOverlap`
  (params (OverlappedComponent :type "PrimitiveComponent Object Reference") (OtherActor :type "Actor Object Reference") (OtherComp :type "PrimitiveComponent Object Reference") (OtherBodyIndex :type Integer) (bFromSweep :type Boolean) (SweepResult :type "HitResult Structure (by ref)"))
  (cast `/Game/BluePrints/BP_BaseHuman` OtherActor)
  (if (`self.CanSpawn`)
    (`|SpawnActorFromClass` "/Game/BluePrints/BP_RandomRocks.BP_RandomRocks_C" (`KismetMathLibrary.MakeTransform` (`self.FallLocation`) (struct) (2.0 2.0 2.0)) "Undefined" "OverrideRootScale" null null)
    (set `self.CanSpawn` false)
    (`KismetSystemLibrary.Delay` 0.2)
    (set `self.CanSpawn` true)
    (if (`self.CanSpawn`)
      (`|SpawnActorFromClass` "/Game/BluePrints/BP_RandomRocks.BP_RandomRocks_C" (`KismetMathLibrary.MakeTransform` (`self.FallLocation3`) (struct) (2.5 2.5 2.5)) "Undefined" "OverrideRootScale" null null)
      (set `self.CanSpawn` false)
      (`KismetSystemLibrary.Delay` 0.5)
      (set `self.CanSpawn` true)
      (if (`self.CanSpawn`)
        (`|SpawnActorFromClass` "/Game/BluePrints/BP_RandomRocks.BP_RandomRocks_C" (`KismetMathLibrary.MakeTransform` (`self.FallLocation2`) (struct) (2.0 2.0 2.0)) "Undefined" "OverrideRootScale" null null)
        (set `self.CanSpawn` false)))))

(fn `UserConstructionScript`)