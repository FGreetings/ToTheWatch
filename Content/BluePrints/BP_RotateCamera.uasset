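; BP_RotateCamera is a box trigger that turns a character and the player's camera rig when a BP_BaseHuman enters it.
; On overlap it rotates the human's capsule 90 degrees, then after a short delay rotates and offsets the Arrow on the BP_Camera1 player pawn.
; The reset logic that would restore both is disconnected, so leaving the box changes nothing.
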(event `self.Box.OnComponentBeginOverlap`
  (params (OverlappedComponent :type "PrimitiveComponent Object Reference") (OtherActor :type "Actor Object Reference") (OtherComp :type "PrimitiveComponent Object Reference") (OtherBodyIndex :type Integer) (bFromSweep :type Boolean) (SweepResult :type "HitResult Structure (by ref)"))
  (bind _asbp_base_human (cast `/Game/BluePrints/BP_BaseHuman` OtherActor))
  (`SceneComponent.K2_SetRelativeRotation` (`Character.CapsuleComponent` _asbp_base_human) (struct :`Yaw` 90.0) false false)
  (`KismetSystemLibrary.Delay` 0.2)
  (bind _asbp_camera_1 (cast `/Game/BluePrints/BP_Camera1` (`GameplayStatics.GetPlayerPawn` 0)))
  (bind _arrow (`/Game/BluePrints/BP_Camera1.Arrow` _asbp_camera_1))
  (`SceneComponent.K2_SetRelativeRotation` _arrow (struct :`Yaw` 90.0) false false)
  (`SceneComponent.K2_SetRelativeLocation` _arrow (100.0 0.0 0.0) false false))

(event `self.Box.OnComponentEndOverlap`
  (params (OverlappedComponent :type "PrimitiveComponent Object Reference") (OtherActor :type "Actor Object Reference") (OtherComp :type "PrimitiveComponent Object Reference") (OtherBodyIndex :type Integer)))

(fn `UserConstructionScript`)