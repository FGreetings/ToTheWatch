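; Player controller for local two-player play on a shared BP_Camera1 pawn, routing both players' move, double-jump and teleport input to two characters.
; BeginPlay spawns both BP_BaseHuman characters at the game instance's BornPosition.
; Tick reads player separation from the camera and updates their relative order.
; Movement follows camera yaw, but past per-axis distance limits only one input direction passes, chosen by that order and IsCamera180, to limit separation.
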(event `self.ReceiveTick`
  (params (DeltaSeconds :type "Float (single-precision)"))
  ;[1 1 1] 获取两玩家之间距离
  (bind _asbp_camera_1 (cast `/Game/BluePrints/BP_Camera1` (`GameplayStatics.GetPlayerPawn` 0)))
  (bind (_playersdistance _playersydistance _playersxdistance) (`/Game/BluePrints/BP_Camera1.GetPlayersDistance` _asbp_camera_1))
  (bind _output_get (set `self.PlayersXDistance` _playersxdistance))
  (bind _output_get_2 (set `self.PlayersYDistance` _playersydistance))
  (`KismetSystemLibrary.PrintString` (`KismetStringLibrary.Concat_StrStr` "x" (`KismetStringLibrary.Conv_DoubleToString` _output_get)))
  (`KismetSystemLibrary.PrintString` (`KismetStringLibrary.Concat_StrStr` "Y:" (`KismetStringLibrary.Conv_DoubleToString` _output_get_2)))
  (`self.ConfirmPlayersLocation`) ; 判断P1P2的相对位置
)

(event `self.ReceiveBeginPlay`
  ;[1 1 1] 初始化
  (`KismetSystemLibrary.Delay` 0.01)
  (bind _asbp_watch_game_instance (cast `/Game/BluePrints/BP_WatchGameInstance` (`GameplayStatics.GetGameInstance`)))
  (bind _bornposition (`/Game/BluePrints/BP_WatchGameInstance.BornPosition` _asbp_watch_game_instance))
  (bind _returnvalue (`AIBlueprintHelperLibrary.SpawnAIFromClass` "/Game/BluePrints/BP_BaseHuman.BP_BaseHuman_C" null (`KismetMathLibrary.MakeVector` (.x _bornposition) (.y _bornposition) (+ (.z _bornposition) 200.0))))
  (bind _asbp_base_human (cast `/Game/BluePrints/BP_BaseHuman` _returnvalue))
  (bind _output_get (set `self.Player1` _asbp_base_human))
  (set `/Game/BluePrints/BP_BaseHuman.IndexOfPlayer` true _output_get)
  (bind _returnvalue_2 (`AIBlueprintHelperLibrary.SpawnAIFromClass` "/Game/BluePrints/BP_BaseHuman.BP_BaseHuman_C" null (`KismetMathLibrary.MakeVector` (+ (.x _bornposition) 200.0) (.y _bornposition) (+ (.z _bornposition) 200.0))))
  (bind _asbp_base_human_2 (cast `/Game/BluePrints/BP_BaseHuman` _returnvalue_2))
  (bind _output_get_2 (set `self.Player2` _asbp_base_human_2))
  (set `/Game/BluePrints/BP_BaseHuman.IndexOfPlayer` false _output_get_2))

(event `InputAxis|MoveForward_p1`
  (params (AxisValue :type "Float (single-precision)"))
  (bind _returnvalue (< AxisValue 0.0))
  (bind _returnvalue_2 (< AxisValue 0.0))
  ;[1 1 1] Player1Movement
  (`/Engine/EditorBlueprintResources/StandardMacros.IsValid` (`self.Player1`)
    (:`Is Valid`
      (if (`self.IsCamera180`)
        (if (< (`self.PlayersYDistance`) 750.0)
          (`/Game/BluePrints/BP_BaseHuman.MoveForward` (`self.Player1`) AxisValue (`KismetMathLibrary.GetForwardVector` (`KismetMathLibrary.MakeRotator` 0.0 0.0 (.yaw (`SceneComponent.K2_GetComponentRotation` (`/Game/BluePrints/BP_Camera1.Arrow` (stale `self.ReceiveTick` _asbp_camera_1)))))) :!label _label)
          (elif (`self.IsP1Front`)
            (if (not _returnvalue_2)
              (goto _label))
            (elif _returnvalue_2
              (goto _label))))
        (elif (< (`self.PlayersYDistance`) 750.0)
          (goto _label)
          (elif (`self.IsP1Front`)
            (if _returnvalue
              (goto _label))
            (elif (not _returnvalue)
              (goto _label))))))))

(event `InputAxis|MoveRight_p1`
  (params (AxisValue :type "Float (single-precision)"))
  (bind _returnvalue (< AxisValue 0.0))
  (bind _isp1right (`self.IsP1Right`))
  ;[1 1 1] Player1Movement
  (`/Engine/EditorBlueprintResources/StandardMacros.IsValid` (`self.Player1`)
    (:`Is Valid`
      (if (`self.IsCamera180`)
        (if (< (`self.PlayersXDistance`) 1100.0)
          (`/Game/BluePrints/BP_BaseHuman.MoveRight` (`self.Player1`) AxisValue (`KismetMathLibrary.GetRightVector` (`KismetMathLibrary.MakeRotator` 0.0 0.0 (.yaw (`SceneComponent.K2_GetComponentRotation` (`/Game/BluePrints/BP_Camera1.Arrow` (stale `self.ReceiveTick` _asbp_camera_1)))))) :!label _label_2)
          (elif _isp1right
            (if _returnvalue
              (goto _label_2))
            (elif (not _returnvalue)
              (goto _label_2))))
        (elif (< (`self.PlayersXDistance`) 1100.0)
          (goto _label_2)
          (elif _isp1right
            (if (not _returnvalue)
              (goto _label_2))
            (elif _returnvalue
              (goto _label_2))))))))

(event `InputAxis|MoveForward_p2`
  (params (AxisValue :type "Float (single-precision)"))
  (bind _returnvalue (< AxisValue 0.0))
  (bind _isp1front (`self.IsP1Front`))
  (bind _returnvalue_2 (< (`self.PlayersYDistance`) 750.0))
  ;[1 1 1] Player2Movement
  (`/Engine/EditorBlueprintResources/StandardMacros.IsValid` (`self.Player2`)
    (:`Is Valid`
      (if (`self.IsCamera180`)
        (if _returnvalue_2
          (`/Game/BluePrints/BP_BaseHuman.MoveForward` (`self.Player2`) AxisValue (`KismetMathLibrary.GetForwardVector` (`KismetMathLibrary.MakeRotator` 0.0 0.0 (.yaw (`SceneComponent.K2_GetComponentRotation` (`/Game/BluePrints/BP_Camera1.Arrow` (stale `self.ReceiveTick` _asbp_camera_1)))))) :!label _label_3)
          (elif _isp1front
            (if _returnvalue
              (goto _label_3))
            (elif (not _returnvalue)
              (goto _label_3))))
        (elif _returnvalue_2
          (goto _label_3)
          (elif _isp1front
            (if (not _returnvalue)
              (goto _label_3))
            (elif _returnvalue
              (goto _label_3))))))))

(event `InputAxis|MoveRight_p2`
  (params (AxisValue :type "Float (single-precision)"))
  (bind _returnvalue (< AxisValue 0.0))
  (bind _isp1right (`self.IsP1Right`))
  (bind _returnvalue_2 (< (`self.PlayersXDistance`) 1100.0))
  ;[1 1 1] Player2Movement
  (`/Engine/EditorBlueprintResources/StandardMacros.IsValid` (`self.Player2`)
    (:`Is Valid`
      (if (`self.IsCamera180`)
        (if _returnvalue_2
          (`/Game/BluePrints/BP_BaseHuman.MoveRight` (`self.Player2`) AxisValue (`KismetMathLibrary.GetRightVector` (`KismetMathLibrary.MakeRotator` 0.0 0.0 (.yaw (`SceneComponent.K2_GetComponentRotation` (`/Game/BluePrints/BP_Camera1.Arrow` (stale `self.ReceiveTick` _asbp_camera_1)))))) :!label _label_4)
          (elif _isp1right
            (if (not _returnvalue)
              (goto _label_4))
            (elif _returnvalue
              (goto _label_4))))
        (elif _returnvalue_2
          (goto _label_4)
          (elif _isp1right
            (if _returnvalue
              (goto _label_4))
            (elif (not _returnvalue)
              (goto _label_4))))))))

(event `InputAction|Jump`
  (params (Key :type "Key Structure"))
  (bind _player1 (`self.Player1`))
  ;[1 1 1] Player1Jump
  (:`Pressed`
    (`/Engine/EditorBlueprintResources/StandardMacros.IsValid` _player1
      (:`Is Valid`
        (`|ExecutionSequence`
          (:`then_0`
            (`Character.Jump` _player1))
          (:`then_1`
            (if (`NavMovementComponent.IsFalling` (`Character.CharacterMovement` _player1))
              (`KismetSystemLibrary.Delay` 0.2)
              (`/Game/BluePrints/BP_BaseHuman.SecondJump` _player1)))))))
  (:`Released`
    (`/Engine/EditorBlueprintResources/StandardMacros.IsValid` _player1
      (:`Is Valid`
        (`Character.StopJumping` _player1)))))

(event `InputAction|Jump_P2`
  (params (Key :type "Key Structure"))
  (bind _player2 (`self.Player2`))
  ;[1 1 1] Player2Jump
  (:`Pressed`
    (`/Engine/EditorBlueprintResources/StandardMacros.IsValid` _player2
      (:`Is Valid`
        (`|ExecutionSequence`
          (:`then_0`
            (`Character.Jump` _player2))
          (:`then_1`
            (if (`NavMovementComponent.IsFalling` (`Character.CharacterMovement` _player2))
              (`KismetSystemLibrary.Delay` 0.2)
              (`/Game/BluePrints/BP_BaseHuman.SecondJump` _player2)))))))
  (:`Released`
    (`/Engine/EditorBlueprintResources/StandardMacros.IsValid` _player2
      (:`Is Valid`
        (`Character.StopJumping` _player2)))))

(event `InputAction|Teleport_p1`
  (params (Key :type "Key Structure"))
  (:`Pressed`
    (`/Game/BluePrints/BP_BaseHuman.Teleport` (`self.Player1`) (`self.Player2`))))

(event `InputAction|Teleport_p2`
  (params (Key :type "Key Structure"))
  (:`Pressed`
    (`/Game/BluePrints/BP_BaseHuman.Teleport` (`self.Player2`) (`self.Player1`))))

(fn `ConfirmPlayersLocation`
  (bind _player1 (`self.Player1`))
  (`/Engine/EditorBlueprintResources/StandardMacros.IsValid` _player1
    (:`Is Valid`
      (set `self.IsP1Front` (> (.y (`self.K2_GetActorLocation` _player1)) (.y (`self.K2_GetActorLocation` (`self.Player2`)))))
      (set `self.IsP1Right` (> (.x (`self.K2_GetActorLocation` _player1)) (.x (`self.K2_GetActorLocation` (`self.Player2`))))))))

(fn `UserConstructionScript`)