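; BP_MachineArms is a Blueprint that rotates two machine arm components to follow the orientation of two reference components, ZL and ZL2.
; Each tick it sets both arms' world rotation using the root's pitch and yaw plus a stored roll.
; It then recomputes each roll as root yaw minus the matching reference's yaw, so that value applies on the following tick.
; The construction script positions only Arm1, at an offset from the root.
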(event `self.ReceiveBeginPlay`)

(event `self.ReceiveTick`
  (params (DeltaSeconds :type "Float (single-precision)"))
  (bind _pitch (.pitch (`SceneComponent.K2_GetComponentRotation` (`self.DefaultSceneRoot`))))
  (bind _yaw (.yaw (`SceneComponent.K2_GetComponentRotation` (`self.DefaultSceneRoot`))))
  (`|ExecutionSequence`
    (:`then_0`
      (`SceneComponent.K2_SetWorldRotation` (`self.Arm1`) (`KismetMathLibrary.MakeRotator` (`self.Arm1_NowRotation_X`) _pitch _yaw) false false)
      (`SceneComponent.K2_SetWorldRotation` (`self.Arm2`) (`KismetMathLibrary.MakeRotator` (`self.Arm2_NowRotation_X`) _pitch _yaw) false false))
    (:`then_1`
      (set `self.Arm1_NowRotation_X` (- _yaw (.yaw (`SceneComponent.K2_GetComponentRotation` (`self.ZL`))))))
    (:`then_2`
      (set `self.Arm2_NowRotation_X` (- _yaw (.yaw (`SceneComponent.K2_GetComponentRotation` (`self.ZL2`))))))))

(fn `UserConstructionScript`
  (`SceneComponent.K2_SetWorldLocation` (`self.Arm1`) (+ (`SceneComponent.K2_GetComponentLocation` (`self.DefaultSceneRoot`)) (`self.Arm1_offset`)) false false))