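; BP_P2GetStuff is an interaction actor that dispenses a stuff item, apparently for one player, as its P2 name suggests.
; When a BP_BaseHuman begins overlapping its Box, it checks that the human's IndexOfPlayer is false and IsUsingPower is true.
; If both hold, GetStuff spawns a BP_StuffBase at the Sphere component's location.
; The power state is only checked at the moment overlap begins.
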(event `self.Box.OnComponentBeginOverlap`
  (params (OverlappedComponent :type "PrimitiveComponent Object Reference") (OtherActor :type "Actor Object Reference") (OtherComp :type "PrimitiveComponent Object Reference") (OtherBodyIndex :type Integer) (bFromSweep :type Boolean) (SweepResult :type "HitResult Structure (by ref)"))
  (bind _asbp_base_human (cast `/Game/BluePrints/BP_BaseHuman` OtherActor))
  (if (`/Game/BluePrints/BP_BaseHuman.IndexOfPlayer` _asbp_base_human)
    _
    (elif (`/Game/BluePrints/BP_BaseHuman.IsUsingPower` _asbp_base_human)
      (`self.GetStuff`))))

(event `GetStuff`
  (`|SpawnActorFromClass` "/Game/BluePrints/BP_StuffBase.BP_StuffBase_C" (`KismetMathLibrary.MakeTransform` (`SceneComponent.K2_GetComponentLocation` (`self.Sphere`))) "Undefined" "OverrideRootScale" null null))

(fn `UserConstructionScript`)