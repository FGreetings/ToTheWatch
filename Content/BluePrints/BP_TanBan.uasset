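; BP_TanBan is a two-player springboard that launches Player 1 upward when Player 2 enters its trigger while using their power.
; P1Trigger tracks whether Player 1 is on the box from the human's boolean player index, clearing on any human's exit and printing debug state.
; P2Trigger checks index, power and that flag, then launches Player 1 through the watch controller, subtracting current velocity for a consistent vertical boost.
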(event `self.P1Trigger.OnComponentBeginOverlap`
  (params (OverlappedComponent :type "PrimitiveComponent Object Reference") (OtherActor :type "Actor Object Reference") (OtherComp :type "PrimitiveComponent Object Reference") (OtherBodyIndex :type Integer) (bFromSweep :type Boolean) (SweepResult :type "HitResult Structure (by ref)"))
  (bind _asbp_base_human (cast `/Game/BluePrints/BP_BaseHuman` OtherActor))
  (bind _output_get (set `self.IsPlayer1OnBox` (`/Game/BluePrints/BP_BaseHuman.IndexOfPlayer` _asbp_base_human)))
  (`KismetSystemLibrary.PrintString` (`KismetStringLibrary.Conv_BoolToString` _output_get)))

(event `self.P1Trigger.OnComponentEndOverlap`
  (params (OverlappedComponent :type "PrimitiveComponent Object Reference") (OtherActor :type "Actor Object Reference") (OtherComp :type "PrimitiveComponent Object Reference") (OtherBodyIndex :type Integer))
  (cast `/Game/BluePrints/BP_BaseHuman` OtherActor)
  (bind _output_get (set `self.IsPlayer1OnBox` false))
  (`KismetSystemLibrary.PrintString` (`KismetStringLibrary.Conv_BoolToString` _output_get)))

(event `self.P2Trigger.OnComponentBeginOverlap`
  (params (OverlappedComponent :type "PrimitiveComponent Object Reference") (OtherActor :type "Actor Object Reference") (OtherComp :type "PrimitiveComponent Object Reference") (OtherBodyIndex :type Integer) (bFromSweep :type Boolean) (SweepResult :type "HitResult Structure (by ref)"))
  (bind _asbp_base_human (cast `/Game/BluePrints/BP_BaseHuman` OtherActor))
  (if (`/Game/BluePrints/BP_BaseHuman.IndexOfPlayer` _asbp_base_human)
    _
    (elif (`/Game/BluePrints/BP_BaseHuman.IsUsingPower` _asbp_base_human)
      (if (`self.IsPlayer1OnBox`)
        (`self.MakePlayer1Fly`)))))

(event `MakePlayer1Fly`
  (bind _asbp_watch_player_controller (cast `/Game/BluePrints/BP_WatchPlayerController` (`GameplayStatics.GetPlayerController` 0)))
  (bind _player1 (`/Game/BluePrints/BP_WatchPlayerController.Player1` _asbp_watch_player_controller))
  (`Character.LaunchCharacter` _player1 (- (0.0 0.0 1200.0) (`self.GetVelocity` _player1)) false false))

(fn `UserConstructionScript`)