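; Base human character for players, providing movement input, a once-per-jump air power and a teleport to another player.
; IndexOfPlayer picks the power: low-gravity float or heavy drop without horizontal velocity.
; Tick clears the using flag when not falling and resets gravity and availability when the jump count is zero.
; Teleport targets the other player's Box on a 15-second cooldown; overlapping a conversation trigger attaches an overhead particle component.
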(event `self.ReceiveTick`
  (params (DeltaSeconds :type "Float (single-precision)"))
  (`|ExecutionSequence`
    (:`then_0`
      (if (not (`NavMovementComponent.IsFalling` (`self.CharacterMovement`)))
        (set `self.IsUsingPower` false)))
    (:`then_1`
      (if (== (`self.JumpCurrentCount`) 0)
        (set `CharacterMovementComponent.GravityScale` 1.0 (`self.CharacterMovement`))
        (set `self.IsPowerUsed` false)))))

(event `MoveForward`
  (params (VAl :type "Float (double-precision)") (WorldDirection :type "Vector Structure"))
  ;[1 1 1] Movement
  (`self.AddMovementInput` WorldDirection VAl))

(event `MoveRight`
  (params (VAL :type "Float (double-precision)") (WorldDirection :type "Vector Structure"))
  ;[1 1 1] Movement
  (`self.AddMovementInput` WorldDirection VAL))

(event `SecondJump`
  (bind _ispowerused (`self.IsPowerUsed`))
  (bind _charactermovement (`self.CharacterMovement`))
  ;[1 1 1] 特殊跳跃技能
  (if (`self.IndexOfPlayer`)
    (if (not _ispowerused)
      (set `CharacterMovementComponent.GravityScale` 0.4 (`self.CharacterMovement`))
      (set `self.IsPowerUsed` true)
      (set `self.IsUsingPower` true)
      (`KismetSystemLibrary.PrintString` "Hello"))
    (elif (not _ispowerused)
      (set `MovementComponent.Velocity` (`KismetMathLibrary.MakeVector` 0.0 0.0 (.z (`self.GetVelocity`))) _charactermovement)
      (set `CharacterMovementComponent.GravityScale` 5.0 _charactermovement)
      (set `self.IsPowerUsed` true)
      (set `self.IsUsingPower` true))))

(event `Teleport`
  (params (`Another Player` :type "/Game/BluePrints/BP_BaseHuman Object Reference"))
  ;[1 1 1] 传送到玩家身后
  (if (`self.CanTeleport`)
    (`self.K2_TeleportTo` self (`SceneComponent.K2_GetComponentLocation` (`/Game/BluePrints/BP_BaseHuman.Box` `Another Player`)) (`SceneComponent.K2_GetComponentRotation` (`self.CapsuleComponent`)))
    (set `self.CanTeleport` false)
    (`KismetSystemLibrary.Delay` 15.0)
    (set `self.CanTeleport` true)))

(event `ShowConversation`)

(event `self.CapsuleComponent.OnComponentBeginOverlap`
  (params (OverlappedComponent :type "PrimitiveComponent Object Reference") (OtherActor :type "Actor Object Reference") (OtherComp :type "PrimitiveComponent Object Reference") (OtherBodyIndex :type Integer) (bFromSweep :type Boolean) (SweepResult :type "HitResult Structure (by ref)"))
  (cast `/Game/BluePrints/BP_ConversationTrigger` OtherActor)
  (bind _returnvalue (`AddComponent|NODE_AddParticleSystemComponent-0` :`RelativeTransform` (`KismetMathLibrary.MakeTransform` (0.0 0.0 150.0))))
  (`SceneComponent.K2_AttachToComponent` _returnvalue (`self.CapsuleComponent`) "None" "KeepRelative" "KeepRelative" "KeepRelative" true))

(fn `UserConstructionScript`)