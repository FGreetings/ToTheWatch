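; Shared camera for two players, whose references it takes from BP_WatchPlayerController shortly after BeginPlay.
; Each Tick it moves to their midpoint with a fixed Y offset, using the higher player's Z.
; Past a horizontal separation threshold, square-root scaling raises it, pushes it along Y and adjusts pitch, unless Player1 is using a power.
; A forward trace meant for fading obstacles has its result unused; the FOV timeline never runs.
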(event `self.ReceiveBeginPlay`
  (`KismetSystemLibrary.Delay` 0.3)
  (bind _asbp_watch_player_controller (cast `/Game/BluePrints/BP_WatchPlayerController` (`GameplayStatics.GetPlayerController` 0)))
  (set `self.Player1` (`/Game/BluePrints/BP_WatchPlayerController.Player1` _asbp_watch_player_controller))
  (set `self.Player2` (`/Game/BluePrints/BP_WatchPlayerController.Player2` _asbp_watch_player_controller)))

(event `self.ReceiveTick`
  (params (DeltaSeconds :type "Float (single-precision)"))
  (bind _player1 (`self.Player1`))
  (bind _player1_2 (`self.Player1`))
  (bind _camerazoffsetinitial (`self.CameraZOffsetInitial`))
  (bind _returnvalue (`SceneComponent.K2_GetComponentLocation` (`self.Camera`)))
  (bind _z (.z (`self.K2_GetActorLocation` self)))
  (bind _z_2 (.z (`SceneComponent.K2_GetComponentLocation` (`Character.CapsuleComponent` _player1))))
  (bind _z_3 (.z (`SceneComponent.K2_GetComponentLocation` (`Character.CapsuleComponent` (`self.Player2`)))))
  (bind _returnvalue_2 (* (`KismetMathLibrary.MultiplyMultiply_FloatFloat` (- (`self.PlayersDistance`) (`self.CameraBeginUp`)) 0.5) 10.0))
  (`|ExecutionSequence`
    (:`then_0`
      ;[1 1 1] 这是跑路的程序大爷的遗产
      (`/Engine/EditorBlueprintResources/StandardMacros.IsValid` _player1
        (:`Is Valid`
          (if (> _z_2 _z_3)
            (set `self.CameraZ` _z_2)
            (else
              (set `self.CameraZ` _z_3)))
          (`self.K2_SetActorLocation` (`KismetMathLibrary.MakeVector` (- (/ (+ (.x (`SceneComponent.K2_GetComponentLocation` (`Character.CapsuleComponent` _player1))) (.x (`SceneComponent.K2_GetComponentLocation` (`Character.CapsuleComponent` (`self.Player2`))))) 2.0) 0.0) (- (/ (+ (.y (`SceneComponent.K2_GetComponentLocation` (`Character.CapsuleComponent` _player1))) (.y (`SceneComponent.K2_GetComponentLocation` (`Character.CapsuleComponent` (`self.Player2`))))) 2.0) 300.0) (+ (`self.CameraZOffSet`) (`self.CameraZ`)))))))
    (:`then_1`
      (`/Engine/EditorBlueprintResources/StandardMacros.IsValid` _player1_2 :!label _label
        (:`Is Valid`
          (if (not (`/Game/BluePrints/BP_BaseHuman.IsUsingPower` _player1_2))
            (`|ExecutionSequence`
              (:`then_0`
                (bind _playersdistance (`self.GetPlayersDistance`)) ; 获取玩家们的水平距离
                (if (> _playersdistance (`self.CameraBeginUp`))
                  (bind _output_get (set `self.CameraZTemp` (+ _z _camerazoffsetinitial)))
                  (if (< _z _output_get)
                    (set `self.CameraZOffSet` (+ _camerazoffsetinitial _returnvalue_2))
                    (`SceneComponent.K2_SetRelativeRotation` (`self.Camera`) (`KismetMathLibrary.MakeRotator` 0.0 (`self.CameraYRotation`)) false false)
                    (`self.K2_SetActorLocation` (`KismetMathLibrary.MakeVector` (.x (`self.K2_GetActorLocation`)) (+ (.y (`self.K2_GetActorLocation`)) (* _returnvalue_2 0.8)) (.z (`self.K2_GetActorLocation`)))))
                  (else
                    (`SceneComponent.K2_SetRelativeRotation` (`self.Camera`) (`KismetMathLibrary.MakeRotator` 0.0 (`self.CameraRotationInital`)) false false))))
              (:`then_1`
                (set `self.CameraYRotation` (+ -40.0 (* _returnvalue_2 -0.1)))))))))
    (:`then_2`
      (goto _label))
    (:`then_3`
      ;[1 1 1] 相机发出射线，检测到的障碍物变透明
      (`KismetSystemLibrary.LineTraceSingle` _returnvalue (+ _returnvalue (* (`KismetMathLibrary.GetForwardVector` (`self.GetControlRotation`)) 1000.0)) "TraceTypeQuery1"))))

(fn `GetPlayersDistance`
  (returns (PlayersDistance :type "Float (double-precision)") (PlayersYDistance :type "Float (double-precision)") (PlayersXDistance :type "Float (double-precision)"))
  (bind _player1 (`self.Player1`))
  (bind _x (.x (`self.K2_GetActorLocation` (`self.Player2`))))
  (bind _y (.y (`self.K2_GetActorLocation` (`self.Player2`))))
  (bind _x_2 (.x (`self.K2_GetActorLocation` _player1)))
  (bind _y_2 (.y (`self.K2_GetActorLocation` _player1)))
  (`/Engine/EditorBlueprintResources/StandardMacros.IsValid` _player1
    (:`Is Valid`
      (bind _output_get (set `self.PlayersDistance` (`KismetMathLibrary.VSize` (- (`KismetMathLibrary.MakeVector` _x_2 _y_2) (`KismetMathLibrary.MakeVector` _x _y)))))
      (bind _output_get_2 (set `self.PlayersYDistance` (`KismetMathLibrary.VSize` (- (`KismetMathLibrary.MakeVector` 0.0 _y_2) (`KismetMathLibrary.MakeVector` 0.0 _y)))))
      (bind _output_get_3 (set `self.PlayersXDistance` (`KismetMathLibrary.VSize` (- (`KismetMathLibrary.MakeVector` _x_2) (`KismetMathLibrary.MakeVector` _x)))))
      (return _output_get _output_get_2 _output_get_3))))

(fn `UserConstructionScript`
  (bind _camera (`self.Camera`))
  (`SceneComponent.K2_SetRelativeRotation` _camera (`KismetMathLibrary.MakeRotator` 0.0 (`self.CameraRotationInital`)) false false)
  (`SceneComponent.K2_SetRelativeLocation` _camera (`self.CameraOffsetInital`) false false)
  (`CameraComponent.SetFieldOfView` (`self.Camera`) (`self.FieldOfView`)))